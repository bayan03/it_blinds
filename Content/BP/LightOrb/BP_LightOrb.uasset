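; BP_LightOrb is an orb pickup that the first-person player can collect only while it is lit.
; The construction script sets material and Niagara auto-activation from IsLit, and the Lightingtheorb event switches it to lit at runtime.
; When the cached player overlaps the sphere of a lit orb, it calls OrbCollected, activates the Niagara component on NiagaraLocation, plays a sound and destroys itself.
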(event `self.ReceiveBeginPlay`
  (bind _asbp_first_person_character (cast `/Game/Starting/FirstPerson/Blueprints/BP_FirstPersonCharacter` (`GameplayStatics.GetPlayerCharacter` 0)))
  (set `self.PlayerRef` _asbp_first_person_character))

(event `self.Sphere.OnComponentBeginOverlap`
  (params (OverlappedComponent :type "PrimitiveComponent Object Reference") (OtherActor :type "Actor Object Reference") (OtherComp :type "PrimitiveComponent Object Reference") (OtherBodyIndex :type Integer) (bFromSweep :type Boolean) (SweepResult :type "HitResult Structure (by ref)"))
  (bind _playerref (`self.PlayerRef`))
  (if (`self.IsLit?`)
    (if (== OtherActor _playerref)
      (`/Game/Starting/FirstPerson/Blueprints/BP_FirstPersonCharacter.Orb Collected` _playerref)
      (`ActorComponent.SetActive` (`NiagaraActor.NiagaraComponent` (`self.niagaraLocation`)) true false)
      (`GameplayStatics.PlaySound2D` "/Game/Sounds/scale-e6-14577.scale-e6-14577" 1.0 1.0 0.0 null null)
      (`self.K2_DestroyActor`))))

(event `Lighting the orb`
  (`PrimitiveComponent.SetMaterial` (`self.StaticMesh`) 0 "/Game/BP/LightOrb/M_LightOrb.M_LightOrb")
  (`ActorComponent.SetActive` (`self.Niagara`) true false)
  (set `self.IsLit?` true))

(fn `UserConstructionScript`
  (bind _niagara (`self.Niagara`))
  (bind _staticmesh (`self.StaticMesh`))
  (if (`self.IsLit?`)
    ;[1 1 1] Activating the orb
    (`ActorComponent.SetAutoActivate` _niagara true)
    (`PrimitiveComponent.SetMaterial` _staticmesh 0 "/Game/BP/LightOrb/M_LightOrb.M_LightOrb")
    (else
      ;[1 1 1] Deactivating the orb
      (`ActorComponent.SetAutoActivate` _niagara false)
      (`PrimitiveComponent.SetMaterial` _staticmesh 0 "/Engine/TemplateResources/MI_Template_BaseGray.MI_Template_BaseGray"))))