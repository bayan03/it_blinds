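; BP_reflection is a Puzzle 1 trigger volume that simulates a mirror reflecting light when the player stands inside it.
; It caches the first-person character on BeginPlay.
; On Box overlap it raises that character's ReflectionLight to a high intensity if the player has the mirror, and zeroes it when the player leaves.
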(event `self.ReceiveBeginPlay`
  (bind _asbp_first_person_character (cast `/Game/Starting/FirstPerson/Blueprints/BP_FirstPersonCharacter` (`GameplayStatics.GetPlayerCharacter` 0)))
  (set `self.Player Ref` _asbp_first_person_character))

(event `self.Box.OnComponentBeginOverlap`
  (params (OverlappedComponent :type "PrimitiveComponent Object Reference") (OtherActor :type "Actor Object Reference") (OtherComp :type "PrimitiveComponent Object Reference") (OtherBodyIndex :type Integer) (bFromSweep :type Boolean) (SweepResult :type "HitResult Structure (by ref)"))
  (bind _player_ref (`self.Player Ref`))
  (if (and (== OtherActor _player_ref) (`/Game/Starting/FirstPerson/Blueprints/BP_FirstPersonCharacter.HasMirror` _player_ref))
    (`LightComponent.SetIntensity` (`/Game/Starting/FirstPerson/Blueprints/BP_FirstPersonCharacter.Reflection light` (`self.Player Ref`)) 200000.0)))

(event `self.Box.OnComponentEndOverlap`
  (params (OverlappedComponent :type "PrimitiveComponent Object Reference") (OtherActor :type "Actor Object Reference") (OtherComp :type "PrimitiveComponent Object Reference") (OtherBodyIndex :type Integer))
  (if (== OtherActor (`self.Player Ref`))
    (`LightComponent.SetIntensity` (`/Game/Starting/FirstPerson/Blueprints/BP_FirstPersonCharacter.Reflection light` (`self.Player Ref`)) 0.0)))

(fn `UserConstructionScript`)