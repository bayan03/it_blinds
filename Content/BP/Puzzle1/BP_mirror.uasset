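; BP_mirror is a pickup mirror for Puzzle1 that the first-person player collects by interacting with it.
; A box overlap toggles the player's ClickInputShow flag while the player is in range.
; The Interaction event sets the player's HasMirror flag, puts the antique standing mirror mesh on the player's MirrorPlace component, then destroys the actor.
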(event `self.ReceiveBeginPlay`
  (bind _asbp_first_person_character (cast `/Game/Starting/FirstPerson/Blueprints/BP_FirstPersonCharacter` (`GameplayStatics.GetPlayerCharacter` 0)))
  (set `self.Player Ref` _asbp_first_person_character))

(event `/Game/BP/Puzzle1/BPI_interaction.Interaction`
  (bind _player_ref (`self.Player Ref`))
  (set `/Game/Starting/FirstPerson/Blueprints/BP_FirstPersonCharacter.HasMirror` true _player_ref)
  (`StaticMeshComponent.SetStaticMesh` (`/Game/Starting/FirstPerson/Blueprints/BP_FirstPersonCharacter.MirrorPlace` _player_ref) "/Game/CustomProps/antique_standing_mirror.antique_standing_mirror")
  (`self.K2_DestroyActor`))

(event `self.Box.OnComponentBeginOverlap`
  (params (OverlappedComponent :type "PrimitiveComponent Object Reference") (OtherActor :type "Actor Object Reference") (OtherComp :type "PrimitiveComponent Object Reference") (OtherBodyIndex :type Integer) (bFromSweep :type Boolean) (SweepResult :type "HitResult Structure (by ref)"))
  (bind _player_ref (`self.Player Ref`))
  (if (== OtherActor _player_ref)
    (set `/Game/Starting/FirstPerson/Blueprints/BP_FirstPersonCharacter.Click Input Show` true _player_ref)))

(event `self.Box.OnComponentEndOverlap`
  (params (OverlappedComponent :type "PrimitiveComponent Object Reference") (OtherActor :type "Actor Object Reference") (OtherComp :type "PrimitiveComponent Object Reference") (OtherBodyIndex :type Integer))
  (bind _player_ref (`self.Player Ref`))
  (if (== OtherActor _player_ref)
    (set `/Game/Starting/FirstPerson/Blueprints/BP_FirstPersonCharacter.Click Input Show` false _player_ref)))

(fn `UserConstructionScript`)