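; Water hazard actor that sends the first-person player back to a respawn point on contact.
; BeginPlay caches the player character reference and creates a user UI widget, which is neither stored nor added to the viewport here.
; Hit and overlap events on the static mesh, plus overlap on a box component, each check for that player and teleport it to the RespawnPoint actor's location.
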(event `self.ReceiveBeginPlay`
  (bind _asbp_first_person_character (cast `/Game/Starting/FirstPerson/Blueprints/BP_FirstPersonCharacter` (`GameplayStatics.GetPlayerCharacter` 0)))
  (set `self.Player Ref` _asbp_first_person_character)
  (`|CreateWidget` "/Game/Widgets/WB_UserUI.WB_UserUI_C"))

(event `self.StaticMesh.OnComponentHit`
  (params (HitComponent :type "PrimitiveComponent Object Reference") (OtherActor :type "Actor Object Reference") (OtherComp :type "PrimitiveComponent Object Reference") (NormalImpulse :type "Vector Structure") (Hit :type "HitResult Structure (by ref)"))
  (if (== OtherActor (`self.Player Ref`))
    (`self.K2_SetActorLocation` (`self.Player Ref`) (`self.K2_GetActorLocation` (`self.respawn point`)) false true)))

(event `self.StaticMesh.OnComponentBeginOverlap`
  (params (OverlappedComponent :type "PrimitiveComponent Object Reference") (OtherActor :type "Actor Object Reference") (OtherComp :type "PrimitiveComponent Object Reference") (OtherBodyIndex :type Integer) (bFromSweep :type Boolean) (SweepResult :type "HitResult Structure (by ref)"))
  (if (== OtherActor (`self.Player Ref`))
    (`self.K2_SetActorLocation` (`self.Player Ref`) (`self.K2_GetActorLocation` (`self.respawn point`)) false true)))

(event `self.Box.OnComponentBeginOverlap`
  (params (OverlappedComponent :type "PrimitiveComponent Object Reference") (OtherActor :type "Actor Object Reference") (OtherComp :type "PrimitiveComponent Object Reference") (OtherBodyIndex :type Integer) (bFromSweep :type Boolean) (SweepResult :type "HitResult Structure (by ref)"))
  (if (== OtherActor (`self.Player Ref`))
    (`self.K2_SetActorLocation` (`self.Player Ref`) (`self.K2_GetActorLocation` (`self.respawn point`)) false true)))

(fn `UserConstructionScript`)